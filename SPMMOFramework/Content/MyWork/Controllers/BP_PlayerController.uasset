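; Player controller that sets up input mapping contexts and the HUD, and turns key presses into hotbar ability activations.
; On local BeginPlay it creates WBP_PlayerHUD, passes it to the pawn, and caches the character and its ability component.
; An AnyKey handler tracks Shift/Ctrl/Alt and looks up "KeyName_Modifiers" strings in HotbarKeybinds.
; The matched value's first two characters become the hotbar and slot IDs for ActivateAbilityInSlot on the character.
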(event Custom|Add%20Default%20Mapping%20Contexts
  (for _array_element (Variables|Default|GetMapping%20Contexts%20To%20Add)
    (Input|AddMappingContext (PlayerController|LocalPlayerSubsystems|GetEnhancedInputLocalPlayerSubsystem) _array_element 0 "(bIgnoreAllPressedKeysUntilRelease=True,bForceImmediately=False,bNotifyUserSettings=False)")))

(event Custom|Create%20HUD
  (bind _returnvalue (UserInterface|CreateWidget "/Game/MyWork/UI/WBP_PlayerHUD.WBP_PlayerHUD_C"))
  (UserInterface|Viewport|AddtoViewport _returnvalue 0)
  (Class|BPIPlayerHUD|SetPlayerHUD(Message) (Game|Player|GetPlayerPawn 0) _returnvalue))

(event EventBeginPlay
  (if (Pawn|IsLocalController)
    (CallFunction|AddDefaultMappingContexts)
    (CallFunction|CreateHUD)
    (bind _asbp_player_character (Utilities|Casting|CastToBP_PlayerCharacter (Game|GetPlayerCharacter 0)))
    (bind _output_get (Variables|Default|SetPlayer%20Character _asbp_player_character))
    (Variables|Default|SetPlayer%20Ability%20Component (Variables|/Game/MyWork/Characters/BP_BaseCharacter.BP_BaseCharacter_C|GetAC_AbilityManager _output_get))))

(event Input|KeyboardEvents|AnyKey
  (params (Key :type Key%20Structure :default "None"))
  (:Pressed
    (CallFunction|PressedModifierKeyCheck Key)
    (if (not (CallFunction|IsKeyAModifier? Key))
      (bind _input_suffix (CallFunction|BuildModifierSuffix))
      (if (.ReturnValue (Utilities|Map|Find (Variables|Default|GetHotbar%20Keybinds) (Utilities|String|Append (Utilities|String|Append (Utilities|String|ToString(Text) (Class|KismetInputLibrary|KeyGetDisplayName Key true)) "_") _input_suffix)))
        (Default|ActivateAbilityinSlot (Variables|Default|GetPlayer%20Character) (Math|Conversions|ToInteger(Byte) (Utilities|Array|Get(acopy) (Utilities|String|GetCharacterArrayfromString (Utilities|String|ToString(Integer) (.Value (Utilities|Map|Find (Variables|Default|GetHotbar%20Keybinds) (Utilities|String|Append (Utilities|String|Append (Utilities|String|ToString(Text) (Class|KismetInputLibrary|KeyGetDisplayName Key true)) "_") _input_suffix))))))) (Math|Conversions|ToInteger(Byte) (Utilities|Array|Get(acopy) (Utilities|String|GetCharacterArrayfromString (Utilities|String|ToString(Integer) (.Value (Utilities|Map|Find (Variables|Default|GetHotbar%20Keybinds) (Utilities|String|Append (Utilities|String|Append (Utilities|String|ToString(Text) (Class|KismetInputLibrary|KeyGetDisplayName Key true)) "_") _input_suffix))))) 1))))))
  (:Released
    (CallFunction|ReleasedModifierKeyCheck Key)))

(fn ConstructionScript)

(fn PressedModifierKeyCheck
  (params (Pressed%20Key :type Key%20Structure :default "None"))
  (if (or (== Pressed%20Key "LeftShift") (== Pressed%20Key "RightShift"))
    (Variables|Default|SetShift%20Held? true))
  (if (or (== Pressed%20Key "LeftControl") (== Pressed%20Key "RightControl"))
    (Variables|Default|SetControl%20Held? true))
  (if (or (== Pressed%20Key "LeftAlt") (== Pressed%20Key "RightAlt"))
    (Variables|Default|SetAlt%20Held? true))
  (if (Math|Boolean|ORBoolean (Variables|Default|GetShift%20Held?) (Variables|Default|GetControl%20Held?) (Variables|Default|GetAlt%20Held?))
    (Variables|Default|SetModifier%20Held? true)))

(fn ReleasedModifierKeyCheck
  (params (Pressed%20Key :type Key%20Structure :default "None"))
  (if (or (== Pressed%20Key "LeftShift") (== Pressed%20Key "RightShift"))
    (Variables|Default|SetShift%20Held? false))
  (if (or (== Pressed%20Key "LeftControl") (== Pressed%20Key "RightControl"))
    (Variables|Default|SetControl%20Held? false))
  (if (or (== Pressed%20Key "LeftAlt") (== Pressed%20Key "RightAlt"))
    (Variables|Default|SetAlt%20Held? false))
  (if (Math|Boolean|ORBoolean (Variables|Default|GetShift%20Held?) (Variables|Default|GetControl%20Held?) (Variables|Default|GetAlt%20Held?))
    (Variables|Default|SetModifier%20Held? false)))

(fn IsKeyAModifier?
  (params (Key :type Key%20Structure :default "None"))
  (return (Math|Boolean|ORBoolean (== Key "LeftShift") (== Key "RightShift") (== Key "LeftControl") (== Key "RightControl") (== Key "LeftAlt") (== Key "RightAlt"))))

(fn BuildModifierSuffix
  (LocalVariables|SetL%20Suffix "")
  (Variables|Default|GetShift%20Held?
    (:then
      (LocalVariables|SetL%20Suffix (Utilities|String|Append (LocalVariables|GetL%20Suffix) "Shift")))
    (:else
      _))
  (Variables|Default|GetControl%20Held?
    (:then
      (LocalVariables|SetL%20Suffix (Utilities|String|Append (LocalVariables|GetL%20Suffix) "Ctrl")))
    (:else
      _))
  (Variables|Default|GetAlt%20Held?
    (:then
      (LocalVariables|SetL%20Suffix (Utilities|String|Append (LocalVariables|GetL%20Suffix) "Alt")))
    (:else
      _))
  (return (LocalVariables|GetL%20Suffix)))