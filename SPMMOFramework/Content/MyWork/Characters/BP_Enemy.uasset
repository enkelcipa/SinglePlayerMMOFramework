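; BP_Enemy is an enemy character Blueprint that sets up its overhead nameplate and health display when play begins.
; After the parent BeginPlay, it casts its Widget component's widget to WBP_Nameplate and initializes it with itself.
; It then fires the ACAttributes HP change event with current and max HP to refresh the bar visuals, a step skipped if the cast fails.
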(event EventBeginPlay
  (bind _ac_attributes (Variables|Default|GetAC_Attributes))
  (|CallParentFunction)
  ;[0.15 0.15 0.15 0.5] Initialise Nameplate
  (bind _aswbp_nameplate (Utilities|Casting|CastToWBP_Nameplate (UserInterface|GetWidget (Variables|Default|GetWidget))))
  (Default|Init:Nameplate _aswbp_nameplate self)
  ;[0.15 0.15 0.15 0.5] Used to update bar visuals
  (Default|CallEvent:HPChange _ac_attributes (Variables|/Game/MyWork/Components/AC_Attributes.AC_Attributes_C|GetCurrent%20HP _ac_attributes) (Variables|/Game/MyWork/Components/AC_Attributes.AC_Attributes_C|GetMax%20HP _ac_attributes)))

(fn ConstructionScript
  (|CallParentFunction))