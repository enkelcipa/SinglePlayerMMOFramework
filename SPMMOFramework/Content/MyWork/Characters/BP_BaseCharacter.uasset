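; BP_BaseCharacter is a base character Blueprint that carries an ACAttributes component for its HP and MP.
; BeginPlay tells ACAttributes to initialise its values.
; Getter functions expose the component, its current HP or MP selected by a resource type (zero for None), and the character's target type.
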(event EventBeginPlay
  (Default|Init:Values (Variables|Default|GetAC_Attributes)))

(fn ConstructionScript)

(fn GetAttributeComponent
  (return (Variables|Default|GetAC_Attributes)))

(fn GetCurrentResourceValue
  (params (Resource :type E_Resources%20Enum :default "NewEnumerator2"))
  (switch Utilities|FlowControl|Switch|SwitchonE_Resources Resource
    (:NewEnumerator2
      (return 0.0))
    (:NewEnumerator0
      (return (Variables|/Game/MyWork/Components/AC_Attributes.AC_Attributes_C|GetCurrent%20HP (Variables|Default|GetAC_Attributes))))
    (:NewEnumerator1
      (return (Variables|/Game/MyWork/Components/AC_Attributes.AC_Attributes_C|GetCurrent%20MP (Variables|Default|GetAC_Attributes))))))

(fn GetTargetType
  (return (Variables|Default|GetTarget%20Type)))