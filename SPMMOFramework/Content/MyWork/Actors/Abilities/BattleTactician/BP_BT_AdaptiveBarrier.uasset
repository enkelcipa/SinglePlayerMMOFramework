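; Battle Tactician Adaptive Barrier ability: a placed area effect that supports party members and harms enemies.
; On placement, it heals party members in the sphere for base potency and damages enemies for half that.
; Overlap events apply healing and damage-reduction statuses to allies and a damage status to enemies, removing them on exit.
; Ending the ability removes the owner's Adaptive Barrier status before running the parent's end logic.
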(event EventBeginPlay)

(event Collision|EventActorBeginOverlap
  (params (OtherActor :type Actor%20Object%20Reference)))

(event EventTick
  (params (DeltaSeconds :type Float%20%28single-precision%29))
  (|CallParentFunction DeltaSeconds) ; This node is disabled and will not be called.\nDrag off pins to build functionality.
)

(event EventPlacedEffect
  (bind _valuepin (Utilities|Set|ForEachLoop(Set) (Variables|Default|GetTargets%20in%20Sphere))
    (:then
      (bind _output_get (Variables|Default|SetActor%20in%20Context _valuepin))
      (bind _party_members (Class|BPIParty|GetPartyMembers(Message) (Variables|Default|GetOwner%20Character)))
      (if (Utilities|Array|ContainsItem _party_members _output_get)
        (bind _attribute_component (Class|BPIAttributeHandling|GetAttributeComponent(Message) (Variables|Default|GetActor%20in%20Context)))
        (Default|ApplyHealthChange _attribute_component true (Variables|Default|GetBase%20Potency))
        (else
          (bind _actor_target_type (Class|BPITargeting|GetTargetType(Message) (Variables|Default|GetActor%20in%20Context)))
          (switch Utilities|FlowControl|Switch|SwitchonE_TargetType _actor_target_type
            (:NewEnumerator2
              (bind _attribute_component_2 (Class|BPIAttributeHandling|GetAttributeComponent(Message) (Variables|Default|GetActor%20in%20Context)))
              (Default|ApplyHealthChange _attribute_component_2 false (* (Variables|Default|GetBase%20Potency) 0.5)))))))))

(event EventBeginOverlapEffect
  (params (Actor :type Actor%20Object%20Reference))
  (bind _status_component (Class|BPIStatusHandling|GetStatusComponent(Message) Actor))
  (bind _party_members (Class|BPIParty|GetPartyMembers(Message) (Variables|Default|GetOwner%20Character)))
  (if (Utilities|Array|ContainsItem _party_members Actor)
    (Default|TryApplyStatus _status_component "/Game/MyWork/Actors/Statuses/BattleTactician/BP_BT_AdaptiveBarrierHealing_Status.BP_BT_AdaptiveBarrierHealing_Status_C" (Variables|Default|GetOwner%20Character) false 0.0)
    (Default|TryApplyStatus _status_component "/Game/MyWork/Actors/Statuses/BattleTactician/BP_BT_AdaptiveBarrierDMGReduction_Status.BP_BT_AdaptiveBarrierDMGReduction_Status_C" (Variables|Default|GetOwner%20Character) false 0.0)
    (else
      (bind _actor_target_type (Class|BPITargeting|GetTargetType(Message) Actor))
      (switch Utilities|FlowControl|Switch|SwitchonE_TargetType _actor_target_type
        (:NewEnumerator2
          (Default|TryApplyStatus _status_component "/Game/MyWork/Actors/Statuses/BattleTactician/BP_BT_AdaptiveBarrierDamage_Status.BP_BT_AdaptiveBarrierDamage_Status_C" (Variables|Default|GetOwner%20Character) false 0.0))))))

(event EventEndOverlapEffect
  (params (Actor :type Actor%20Object%20Reference))
  (bind _status_component (Class|BPIStatusHandling|GetStatusComponent(Message) Actor))
  (bind _party_members (Class|BPIParty|GetPartyMembers(Message) (Variables|Default|GetOwner%20Character)))
  (if (Utilities|Array|ContainsItem _party_members Actor)
    (for _array_element (Variables|/Game/MyWork/Components/AC_StatusManager.AC_StatusManager_C|GetActive%20Statuses _status_component)
      (if (== (Utilities|GetClass _array_element) "/Game/MyWork/Actors/Statuses/BattleTactician/BP_BT_AdaptiveBarrierDMGReduction_Status.BP_BT_AdaptiveBarrierDMGReduction_Status_C")
        (Default|RemoveStatus _status_component _array_element)))
    (for _array_element_2 (Variables|/Game/MyWork/Components/AC_StatusManager.AC_StatusManager_C|GetActive%20Statuses _status_component)
      (if (== (Utilities|GetClass _array_element_2) "/Game/MyWork/Actors/Statuses/BattleTactician/BP_BT_AdaptiveBarrierHealing_Status.BP_BT_AdaptiveBarrierHealing_Status_C")
        (Default|RemoveStatus _status_component _array_element_2)))
    (else
      (bind _actor_target_type (Class|BPITargeting|GetTargetType(Message) Actor))
      (switch Utilities|FlowControl|Switch|SwitchonE_TargetType _actor_target_type
        (:NewEnumerator2
          (for _array_element_3 (Variables|/Game/MyWork/Components/AC_StatusManager.AC_StatusManager_C|GetActive%20Statuses _status_component)
            (if (== (Utilities|GetClass _array_element_3) "/Game/MyWork/Actors/Statuses/BattleTactician/BP_BT_AdaptiveBarrierDamage_Status.BP_BT_AdaptiveBarrierDamage_Status_C")
              (Default|RemoveStatus _status_component _array_element_3))))))))

(event EventAbilityEnd
  (bind _status_component (Class|BPIStatusHandling|GetStatusComponent(Message) (Variables|Default|GetOwner%20Character)))
  (for _array_element (Variables|/Game/MyWork/Components/AC_StatusManager.AC_StatusManager_C|GetActive%20Statuses _status_component)
    (if (== (Utilities|GetClass _array_element) "/Game/MyWork/Actors/Statuses/BattleTactician/BP_BT_AdaptiveBarrier_Status.BP_BT_AdaptiveBarrier_Status_C")
      (Default|RemoveStatus _status_component _array_element)))
  (|CallParentFunction))

(fn ConstructionScript
  (|CallParentFunction))