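; Base single-target GCD ability that changes the target's health, then applies statuses to it.
; ApplyEffects sends healing and base potency (as incoming damage) to the target's attribute component.
; It then gets the target's status component via a message call and tries to apply each entry in StatusToApply, with the owner as instigator and a shield potency override, before ending the ability.
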(event EventApplyEffects
  (Default|ApplyHealthChange (Variables|Default|GetTarget%20Attribute%20Component) (Variables|Default|GetHealing?) (Variables|Default|GetBase%20Potency))
  (bind _status_component (Class|BPIStatusHandling|GetStatusComponent(Message) (Variables|Default|GetTarget)))
  (Variables|Default|SetTarget%20Status%20Component _status_component)
  (for _array_element (Variables|Default|GetStatus'%20to%20Apply)
    (Default|TryApplyStatus (Variables|Default|GetTarget%20Status%20Component) _array_element (Variables|Default|GetOwner%20Character) (Variables|Default|GetOverride%20Shield%20Potency?) (Variables|Default|GetOverride%20Shield%20Potency)))
  (CallFunction|AbilityEnd))

(fn ConstructionScript
  (|CallParentFunction))