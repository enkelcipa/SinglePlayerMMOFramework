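; Base GCD area-of-effect ability that changes health, then applies statuses to characters around the target.
; ApplyEffects runs a sphere overlap of AbilityRadius at the Target's location, keeping BP_BaseCharacter pawns whose target type is in TargetType.
; Each match receives healing or damage through its attribute component, then every StatusToApply entry through its status component with the owner as instigator.
; The ability ends once all overlapped actors are processed.
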(event EventApplyEffects
  (bind _outactors (Collision|SphereOverlapActors (Transformation|GetActorLocation (Variables|Default|GetTarget)) (Variables|Default|GetAbility%20Radius) (Utilities|Array|MakeArray "ObjectTypeQuery3") "/Game/MyWork/Characters/BP_BaseCharacter.BP_BaseCharacter_C"))
  (for _array_element _outactors
    (bind _actor_target_type (Class|BPITargeting|GetTargetType(Message) _array_element))
    (if (Utilities|Array|ContainsItem (Variables|Default|GetTarget%20Type) _actor_target_type)
      (bind _attribute_component (Class|BPIAttributeHandling|GetAttributeComponent(Message) _array_element))
      (Default|ApplyHealthChange _attribute_component (Variables|Default|GetHealing?) (Variables|Default|GetBase%20Potency))
      (bind _status_component (Class|BPIStatusHandling|GetStatusComponent(Message) _array_element))
      (Variables|Default|SetTarget%20Status%20Component _status_component)
      (for _array_element_2 (Variables|Default|GetStatus'%20to%20Apply)
        (Default|TryApplyStatus (Variables|Default|GetTarget%20Status%20Component) _array_element_2 (Variables|Default|GetOwner%20Character) (Variables|Default|GetOverride%20Shield%20Potency?) (Variables|Default|GetOverride%20Shield%20Potency)))))
  (CallFunction|AbilityEnd))

(fn ConstructionScript
  (|CallParentFunction))