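; A global-cooldown cast ability that deals area damage around its target.
; On ApplyEffects it sphere-overlaps pawns of the base character class within the ability radius at the target's location.
; It keeps actors whose target type, read through an interface message, is in the ability's allowed types, then applies base potency as damage through each one's attribute component.
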(event EventApplyEffects
  (bind _outactors (Collision|SphereOverlapActors (Transformation|GetActorLocation (Variables|Default|GetTarget)) (Variables|Default|GetAbility%20Radius) (Utilities|Array|MakeArray "ObjectTypeQuery3") "/Game/MyWork/Characters/BP_BaseCharacter.BP_BaseCharacter_C"))
  (for _array_element _outactors
    (bind _actor_target_type (Class|BPITargeting|GetTargetType(Message) _array_element))
    (if (Utilities|Array|ContainsItem (Variables|Default|GetTarget%20Type) _actor_target_type)
      (bind _attribute_component (Class|BPIAttributeHandling|GetAttributeComponent(Message) _array_element))
      (Default|ApplyHealthChange _attribute_component false (Variables|Default|GetBase%20Potency)))))

(fn ConstructionScript
  (|CallParentFunction))