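; Base area-of-effect oGCD ability that changes the health of the owner's party members within a radius.
; ApplyEffects sphere-overlaps base character pawns around the owner and keeps only those in the owner's party list.
; Each match's attribute component receives the base potency with the Healing flag, then the ability ends.
; The party filter applies regardless of that flag, so non-party characters are never affected.
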(event EventBeginPlay
  (|CallParentFunction) ; This node is disabled and will not be called.\nDrag off pins to build functionality.
)

(event EventApplyEffects
  (bind _outactors (Collision|SphereOverlapActors (Transformation|GetActorLocation (Variables|Default|GetOwner%20Character)) (Variables|Default|GetAbility%20Radius) (Utilities|Array|MakeArray "ObjectTypeQuery3") "/Game/MyWork/Characters/BP_BaseCharacter.BP_BaseCharacter_C"))
  (for _array_element _outactors
    (bind _party_members (Class|BPIParty|GetPartyMembers(Message) (Variables|Default|GetOwner%20Character)))
    (if (Utilities|Array|ContainsItem _party_members _array_element)
      (bind _attribute_component (Class|BPIAttributeHandling|GetAttributeComponent(Message) _array_element))
      (Default|ApplyHealthChange _attribute_component (Variables|Default|GetHealing?) (Variables|Default|GetBase%20Potency))))
  (CallFunction|AbilityEnd))

(fn ConstructionScript
  (|CallParentFunction))