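; Base oGCD self-targeted ability that toggles the owning character between a primary and a secondary set of statuses.
; ApplyEffects gets the owner's status component and uses the Active flag to choose which set to remove and which to apply.
; It removes active statuses by exact class match, applies the other set with the owner as instigator, then flips Active and ends the ability.
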(event EventBeginPlay
  (|CallParentFunction) ; This node is disabled and will not be called.\nDrag off pins to build functionality.
)

(event EventApplyEffects
  (bind _status_component (Class|BPIStatusHandling|GetStatusComponent(Message) (Variables|Default|GetOwner%20Character)))
  (Variables|Default|SetTarget%20Status%20Component _status_component)
  (if (Variables|Default|GetActive?)
    ;[0.15 0.15 0.15 0.5] Remove Primary Status' and add Secondary ones
    (for _array_element (Variables|Default|GetStatus'%20to%20Apply)
      (bind _valuepin (Utilities|Set|ForEachLoop(Set) (Variables|/Game/MyWork/Components/AC_StatusManager.AC_StatusManager_C|GetActive%20Statuses (Variables|Default|GetTarget%20Status%20Component)))
        (:then
          (if (== (Utilities|GetClass _valuepin) _array_element)
            (Default|RemoveStatus (Variables|Default|GetTarget%20Status%20Component) _valuepin)))))
    (for _array_element_2 (Variables|Default|GetSecondary%20Status'%20to%20Apply)
      (Default|TryApplyStatus (Variables|Default|GetTarget%20Status%20Component) _array_element_2 (Variables|Default|GetOwner%20Character)))
    (Variables|Default|SetActive? false)
    (CallFunction|AbilityEnd)
    (else
      ;[0.15 0.15 0.15 0.5] Remove Secondary Status' and add Primary ones
      (for _array_element_3 (Variables|Default|GetSecondary%20Status'%20to%20Apply)
        (bind _valuepin_2 (Utilities|Set|ForEachLoop(Set) (Variables|/Game/MyWork/Components/AC_StatusManager.AC_StatusManager_C|GetActive%20Statuses (Variables|Default|GetTarget%20Status%20Component)))
          (:then
            (if (== (Utilities|GetClass _valuepin_2) _array_element_3)
              (Default|RemoveStatus (Variables|Default|GetTarget%20Status%20Component) _valuepin_2)))))
      (for _array_element_4 (Variables|Default|GetStatus'%20to%20Apply)
        (Default|TryApplyStatus (Variables|Default|GetTarget%20Status%20Component) _array_element_4 (Variables|Default|GetOwner%20Character)))
      (Variables|Default|SetActive? true)
      (CallFunction|AbilityEnd))))

(fn ConstructionScript
  (|CallParentFunction))