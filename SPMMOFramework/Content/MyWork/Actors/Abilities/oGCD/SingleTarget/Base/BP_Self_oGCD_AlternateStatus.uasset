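; Base self-targeted oGCD ability that toggles the owner between a primary and a secondary set of statuses.
; ApplyEffects gets the owner's status component and branches on an Active flag.
; Each use removes active statuses whose class exactly matches one set, applies the other set with the owner as instigator, flips Active, then ends the ability.
; Active is true while the primary StatusToApply set is on, so a use from inactive applies that set.
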(event EventBeginPlay
  (|CallParentFunction) ; This node is disabled and will not be called.\nDrag off pins to build functionality.
)

(event EventApplyEffects
  (bind _status_component (Class|BPIStatusHandling|GetStatusComponent(Message) (Variables|Default|GetOwner%20Character)))
  (Variables|Default|SetTarget%20Status%20Component _status_component)
  (if (Variables|Default|GetActive?)
    ;[0.15 0.15 0.15 0.5] Remove Primary Status' and add Secondary ones
    (for _array_element (Variables|Default|GetStatus'%20to%20Apply)
      (for _array_element_2 (Variables|/Game/MyWork/Components/AC_StatusManager.AC_StatusManager_C|GetActive%20Statuses (Variables|Default|GetTarget%20Status%20Component))
        (if (== (Utilities|GetClass _array_element_2) _array_element)
          (Default|RemoveStatus (Variables|Default|GetTarget%20Status%20Component) _array_element_2))))
    (for _array_element_3 (Variables|Default|GetSecondary%20Status'%20to%20Apply)
      (Default|TryApplyStatus (Variables|Default|GetTarget%20Status%20Component) _array_element_3 (Variables|Default|GetOwner%20Character) false 0.0))
    (Variables|Default|SetActive? false)
    (CallFunction|AbilityEnd)
    (else
      ;[0.15 0.15 0.15 0.5] Remove Secondary Status' and add Primary ones
      (for _array_element_4 (Variables|Default|GetSecondary%20Status'%20to%20Apply)
        (for _array_element_5 (Variables|/Game/MyWork/Components/AC_StatusManager.AC_StatusManager_C|GetActive%20Statuses (Variables|Default|GetTarget%20Status%20Component))
          (if (== (Utilities|GetClass _array_element_5) _array_element_4)
            (Default|RemoveStatus (Variables|Default|GetTarget%20Status%20Component) _array_element_5))))
      (for _array_element_6 (Variables|Default|GetStatus'%20to%20Apply)
        (Default|TryApplyStatus (Variables|Default|GetTarget%20Status%20Component) _array_element_6 (Variables|Default|GetOwner%20Character) false 0.0))
      (Variables|Default|SetActive? true)
      (CallFunction|AbilityEnd))))

(fn ConstructionScript
  (|CallParentFunction))