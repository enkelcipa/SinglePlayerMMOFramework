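; Self-targeted oGCD ability base that toggles a list of statuses on its owning character.
; ApplyEffects gets the owner's status component, then for each class in StatusToApply either applies it or removes active statuses of that exact class, based on the Active flag.
; Active flips inside that loop, so consecutive entries alternate between apply and remove.
; The ability ends through AbilityEnd afterward.
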(event EventBeginPlay
  (|CallParentFunction) ; This node is disabled and will not be called.\nDrag off pins to build functionality.
)

(event EventApplyEffects
  (bind _status_component (Class|BPIStatusHandling|GetStatusComponent(Message) (Variables|Default|GetOwner%20Character)))
  (Variables|Default|SetTarget%20Status%20Component _status_component)
  (for _array_element (Variables|Default|GetStatus'%20to%20Apply)
    (if (Variables|Default|GetActive?)
      (bind _valuepin (Utilities|Set|ForEachLoop(Set) (Variables|/Game/MyWork/Components/AC_StatusManager.AC_StatusManager_C|GetActive%20Statuses (Variables|Default|GetTarget%20Status%20Component)))
        (:then
          (if (== (Utilities|GetClass _valuepin) _array_element)
            (Default|RemoveStatus (Variables|Default|GetTarget%20Status%20Component) _valuepin)))
        (:CompletedPin
          (Variables|Default|SetActive? false)))
      (else
        (Default|TryApplyStatus (Variables|Default|GetTarget%20Status%20Component) _array_element (Variables|Default|GetOwner%20Character))
        (Variables|Default|SetActive? true))))
  (CallFunction|AbilityEnd))

(fn ConstructionScript
  (|CallParentFunction))