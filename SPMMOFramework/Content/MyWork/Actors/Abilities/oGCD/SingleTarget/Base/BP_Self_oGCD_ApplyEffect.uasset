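; Base Blueprint for a self-targeted oGCD ability that applies status effects to its owner.
; Its ApplyEffects event gets the owner character's status component through a GetStatusComponentMessage call.
; It tries to apply each entry in StatusToApply with the owner as instigator, then ends the ability.
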(event EventBeginPlay
  (|CallParentFunction) ; This node is disabled and will not be called.\nDrag off pins to build functionality.
)

(event EventApplyEffects
  (bind _status_component (Class|BPIStatusHandling|GetStatusComponent(Message) (Variables|Default|GetOwner%20Character)))
  (Variables|Default|SetTarget%20Status%20Component _status_component)
  (for _array_element (Variables|Default|GetStatus'%20to%20Apply)
    (Default|TryApplyStatus (Variables|Default|GetTarget%20Status%20Component) _array_element (Variables|Default|GetOwner%20Character) false 0.0))
  (CallFunction|AbilityEnd))

(fn ConstructionScript
  (|CallParentFunction))