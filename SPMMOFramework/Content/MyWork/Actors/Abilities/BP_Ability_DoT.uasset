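; Damage-over-time ability actor that deals an initial hit and sets up periodic damage on its target.
; ApplyEffects starts a Duration timer and a looping DOTTickRate timer, then applies BasePotency damage through TargetAttributeComponent.
; ApplyDamage deals DOTPotency damage through the same component's ApplyHealthChange.
; BeginPlay and construction only call the parent implementations.
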(event Custom|Apply%20Damage
  (Default|ApplyHealthChange (Variables|Default|GetTarget%20Attribute%20Component) false (Variables|Default|GetDOT%20Potency)))

(event EventBeginPlay
  (|CallParentFunction))

(event EventApplyEffects
  (Utilities|Time|SetTimerbyEvent (EventDispatchers|CreateEvent :!event AbilityEnd) (Variables|Default|GetDuration))
  (Utilities|Time|SetTimerbyEvent (EventDispatchers|CreateEvent :!event Custom|Apply%20Damage) (Variables|Default|GetDOT%20Tick%20Rate) true)
  (Default|ApplyHealthChange (Variables|Default|GetTarget%20Attribute%20Component) false (Variables|Default|GetBase%20Potency)))

(fn ConstructionScript
  (|CallParentFunction))