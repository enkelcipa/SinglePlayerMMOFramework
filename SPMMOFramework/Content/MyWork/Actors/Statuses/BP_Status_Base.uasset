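; Base actor for status effects applied to a target, with duration and stack tracking for child statuses.
; Init caches the target's attribute and status components through message calls, then sets the duration from StatusData, flagging non-positive durations as infinite.
; Duration resets notify the status component, and adding a stack caps at the maximum and refreshes the duration.
; ApplyStatusEffects is an empty hook; StatusEnd clears the tick timer and destroys the actor.
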(event Custom|Init:%20Status
  (params (Owner :type Character%20Object%20Reference) (Target :type Actor%20Object%20Reference))
  (Variables|Owner|SetOnwer Owner)
  (bind _output_get (Variables|Targeting|SetTarget Target))
  (bind _attribute_component (Class|BPIAttributeHandling|GetAttributeComponent(Message) _output_get))
  (Variables|Targeting|SetTarget%20Attribute%20Component _attribute_component)
  (bind _status_component (Class|BPIStatusHandling|GetStatusComponent(Message) (Variables|Targeting|GetTarget)))
  (Variables|Targeting|SetStatus%20Component _status_component)
  (CallFunction|SetStatusDuration)
  (Variables|Default|SetInfinite%20Duration? (not (> (.BaseDuration (Utilities|Struct|BreakS_StatusDefinition (Variables|StatusData|GetStatus%20Data))) 0.0))))

(event Custom|Set%20Status%20Duration
  (bind _output_get (Variables|StatusData|SetDuration%20Remaining (Math|Float|Truncate (.BaseDuration (Utilities|Struct|BreakS_StatusDefinition (Variables|StatusData|GetStatus%20Data))))))
  (Default|CallEvent:StatusUpdated (Variables|Targeting|GetStatus%20Component) self _output_get))

(event Custom|Status%20End
  (Utilities|Time|ClearandInvalidateTimerbyHandle (Variables|Timers|GetStatus%20Effect%20Tick%20Timer))
  (Actor|DestroyActor))

(event Custom|Apply%20Status%20Effects)

(event Custom|Tick%20Status%20Duration
  (Variables|Default|GetInfinite%20Duration?
    (:then)
    (:else
      (Math|Integer|DecrementInt (Variables|StatusData|GetDuration%20Remaining)))))

(event Custom|Refresh%20Status
  (CallFunction|SetStatusDuration))

(event Custom|Increase%20Stacks
  (Variables|StatusData|SetStacks (Math|Integer|Min(Integer) (+ (Variables|StatusData|GetStacks) 1) (.MaxStacks (Utilities|Struct|BreakS_StatusDefinition (Variables|StatusData|GetStatus%20Data)))))
  (CallFunction|RefreshStatus))

(fn ConstructionScript)