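; Base status effect actor for effects that act periodically over time.
; Extends the parent's duration setup with a one-shot timer using the first tick delay from StatusData.
; StartStatusTicks runs a looping timer at the status tick interval and stores its handle in StatusEffectTickTimer.
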(event Custom|Start%20Status%20Ticks
  (bind _returnvalue (Utilities|Time|SetTimerbyEvent (EventDispatchers|CreateEvent :!event ApplyStatusEffects) (.StatusTickInterval (Utilities|Struct|BreakS_StatusDefinition (Variables|Default|GetStatus%20Data))) true))
  (Variables|Default|SetStatus%20Effect%20Tick%20Timer _returnvalue))

(event EventBeginPlay
  (|CallParentFunction))

(event EventSetStatusDuration
  (|CallParentFunction)
  (Utilities|Time|SetTimerbyEvent (EventDispatchers|CreateEvent :!event Custom|Start%20Status%20Ticks) (.FirstTickDelay (Utilities|Struct|BreakS_StatusDefinition (Variables|Default|GetStatus%20Data)))))

(fn ConstructionScript
  (|CallParentFunction))