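; Base actor for gameplay statuses applied to a target, with duration, stacking, refresh and chance-based procs driven by StatusData.
; Init fetches the target's attribute and status components via interface messages, reports the duration and applies effects immediately unless an over-time effect is set.
; Stack increases are capped and refresh the duration; ending clears the effect timer and destroys the actor.
; Proc effect and shield potency override are empty hooks.
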(event Custom|Init:%20Status
  (params (Owner :type Character%20Object%20Reference) (Target :type Actor%20Object%20Reference) (Override%20Shield%20Potency? :type Boolean) (Override%20Shield%20Potency :type Float%20%28double-precision%29))
  (Variables|Owner|SetOnwer Owner)
  (bind _output_get (Variables|Targeting|SetTarget Target))
  (bind _attribute_component (Class|BPIAttributeHandling|GetAttributeComponent(Message) _output_get))
  (Variables|Targeting|SetTarget%20Attribute%20Component _attribute_component)
  (bind _status_component (Class|BPIStatusHandling|GetStatusComponent(Message) (Variables|Targeting|GetTarget)))
  (Variables|Targeting|SetStatus%20Component _status_component)
  (CallFunction|SetStatusDuration)
  (if Override%20Shield%20Potency?
    (CallFunction|OverrideShieldPotency Override%20Shield%20Potency? Override%20Shield%20Potency))
  (Variables|StatusData|SetInfinite%20Duration? (not (> (Utilities|Struct|BreakS_StatusDefinition (Variables|StatusData|GetStatus%20Data)) 0.0)))
  (Variables|StatusData|GetOver%20Time%20Effect?
    (:then)
    (:else
      (CallFunction|ApplyStatusEffects))))

(event Custom|Set%20Status%20Duration
  (bind _output_get (Variables|StatusData|SetDuration%20Remaining (Math|Float|Truncate (Utilities|Struct|BreakS_StatusDefinition (Variables|StatusData|GetStatus%20Data)))))
  (Default|CallEvent:StatusUpdated (Variables|Targeting|GetStatus%20Component) self _output_get))

(event Custom|Status%20End
  (Utilities|Time|ClearandInvalidateTimerbyHandle (Variables|Timers|GetStatus%20Effect%20Tick%20Timer))
  (Actor|DestroyActor))

(event Custom|Apply%20Status%20Effects
  (if (Math|Random|RandomBoolwithWeight (Utilities|Struct|BreakS_StatusDefinition (Variables|StatusData|GetStatus%20Data)))
    (CallFunction|ApplyProcEffect)))

(event Custom|Tick%20Status%20Duration
  (Variables|StatusData|GetInfinite%20Duration?
    (:then)
    (:else
      (Math|Integer|DecrementInt (Variables|StatusData|GetDuration%20Remaining)))))

(event Custom|Apply%20Proc%20Effect)

(event Custom|Override%20Shield%20Potency
  (params (Override%20Shield%20Potency? :type Boolean) (Override%20Shield%20Potency :type Float%20%28double-precision%29)))

(event Custom|Refresh%20Status
  (CallFunction|SetStatusDuration))

(event Custom|Increase%20Stacks
  (Variables|StatusData|SetStacks (Math|Integer|Min(Integer) (+ (Variables|StatusData|GetStacks) 1) (Utilities|Struct|BreakS_StatusDefinition (Variables|StatusData|GetStatus%20Data))))
  (CallFunction|RefreshStatus))

(fn ConstructionScript)