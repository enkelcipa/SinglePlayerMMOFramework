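; Base status effect actor that grants a shield to its target's attribute component.
; On BeginPlay it records itself as the status actor in its shield struct before running parent logic.
; When effects apply, it passes that shield to TryAddShield, along with an optional potency override that a separate event stores beforehand.
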(event EventBeginPlay
  (Utilities|Struct|SetmembersinS_ShieldInstance (Variables|ShieldingData|GetShield%20to%20Apply) self)
  (|CallParentFunction))

(event EventOverrideShieldPotency
  (params (Override%20Shield%20Potency? :type Boolean) (Override%20Shield%20Potency :type Float%20%28double-precision%29))
  (Variables|ShieldingData|SetOverride%20Shield%20Potency? Override%20Shield%20Potency?)
  (Variables|ShieldingData|SetOverride%20Potency Override%20Shield%20Potency))

(event EventApplyStatusEffects
  (Default|TryAddShield (Variables|Default|GetTarget%20Attribute%20Component) (Variables|ShieldingData|GetShield%20to%20Apply) (Variables|ShieldingData|GetOverride%20Shield%20Potency?) (Variables|ShieldingData|GetOverride%20Potency)))

(fn ConstructionScript
  (|CallParentFunction))