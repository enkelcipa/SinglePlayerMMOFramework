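; Battle Tactician Paradigm Soothe status that heals the most injured party member near its owner.
; When status effects apply, a sphere overlap around the owner gathers characters and keeps those in the owner's party.
; FindLowestHPTarget compares their HP percentages and returns the lowest one's attribute component, which receives healing equal to the status's base potency.
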(event EventBeginPlay
  (|CallParentFunction) ; This node is disabled and will not be called.\nDrag off pins to build functionality.
)

(event EventApplyStatusEffects
  (bind _lowest_hp__actor (CallFunction|FindLowestHPTarget))
  ;[0.15 0.15 0.15 0.5] Clear array before doing anything
  (Utilities|Array|Clear (Variables|Default|GetTargets%20in%20Range))
  ;[0.15 0.15 0.15 0.5] Overlap for all BP_BaseCharacters in range
  (bind _outactors (Collision|SphereOverlapActors (Transformation|GetActorLocation (Variables|Default|GetOnwer)) (Variables|Default|GetRadius) (Utilities|Array|MakeArray "ObjectTypeQuery3") "/Game/MyWork/Characters/BP_BaseCharacter.BP_BaseCharacter_C"))
  ;[0.15 0.15 0.15 0.5] For each actor, check if they are in the party
  (for _array_element _outactors
    (bind _party_members (Class|BPIParty|GetPartyMembers(Message) (Variables|Default|GetOnwer)))
    ;[0.15 0.15 0.15 0.5] If they are, add to the Targets in Range array
    (if (Utilities|Array|ContainsItem _party_members _array_element)
      (Utilities|Array|Add (Variables|Default|GetTargets%20in%20Range) _array_element)))
  (Utilities|IsValid _lowest_hp__actor
    (:Is%20Valid
      (Default|ApplyHealthChange _lowest_hp__actor (Variables|Default|GetHealing?) (Utilities|Struct|BreakS_StatusDefinition (Variables|Default|GetStatus%20Data))))))

(fn ConstructionScript
  (|CallParentFunction))

(fn FindLowestHPTarget
  (for _array_element (Variables|Default|GetTargets%20in%20Range)
    (bind _attribute_component (Class|BPIAttributeHandling|GetAttributeComponent(Message) _array_element))
    (if (< (|((CurrentHP/MaxHP)*100) (Variables|/Game/MyWork/Components/AC_Attributes.AC_Attributes_C|GetCurrent%20HP _attribute_component) (Variables|/Game/MyWork/Components/AC_Attributes.AC_Attributes_C|GetMax%20HP _attribute_component)) (LocalVariables|GetL%20Current%20Lowest%20HP))
      (LocalVariables|SetL%20Current%20Lowest%20HP (|((CurrentHP/MaxHP)*100) (Variables|/Game/MyWork/Components/AC_Attributes.AC_Attributes_C|GetCurrent%20HP _attribute_component) (Variables|/Game/MyWork/Components/AC_Attributes.AC_Attributes_C|GetMax%20HP _attribute_component)))
      (LocalVariables|SetL%20Target%20with%20Lowest%20HP _attribute_component)))
  (return (LocalVariables|GetL%20Target%20with%20Lowest%20HP)))