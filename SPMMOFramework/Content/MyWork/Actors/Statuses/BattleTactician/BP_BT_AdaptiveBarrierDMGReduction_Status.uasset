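; Battle Tactician status actor that grants its owner damage reduction, named for the Adaptive Barrier.
; On applying its effects, it adds a multiplicative mitigation to the owner's attribute component, registering itself as the source.
; When the status ends, it removes the mitigation by that same source and then runs the parent's end logic.
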(event EventBeginPlay)

(event Collision|EventActorBeginOverlap
  (params (OtherActor :type Actor%20Object%20Reference)))

(event EventTick
  (params (DeltaSeconds :type Float%20%28single-precision%29)))

(event EventApplyStatusEffects
  (bind _attribute_component (Class|BPIAttributeHandling|GetAttributeComponent(Message) (Variables|Default|GetOnwer)))
  (Default|AddMitigation _attribute_component 0.9 self))

(event EventStatusEnd
  (bind _attribute_component (Class|BPIAttributeHandling|GetAttributeComponent(Message) (Variables|Default|GetOnwer)))
  (Default|RemoveMitigation _attribute_component self)
  (|CallParentFunction))

(fn ConstructionScript
  (|CallParentFunction))