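; Battle Tactician Paradigm Harm status effect that applies a health change to the closest enemy around its owner.
; When applied, it sphere-overlaps pawns within Radius and keeps BP_BaseCharacters whose target-type message marks them as enemies.
; FindClosestTarget picks the nearest one's attribute component, which receives the status's base potency and Healing flag through ApplyHealthChange.
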(event EventBeginPlay
  (|CallParentFunction) ; This node is disabled and will not be called.\nDrag off pins to build functionality.
)

(event EventApplyStatusEffects
  (bind _closest_actor (CallFunction|FindClosestTarget))
  ;[0.15 0.15 0.15 0.5] Clear array before doing anything
  (Utilities|Array|Clear (Variables|Default|GetTargets%20in%20Range))
  ;[0.15 0.15 0.15 0.5] Overlap for all BP_BaseCharacters in range
  (bind _outactors (Collision|SphereOverlapActors (Transformation|GetActorLocation (Variables|Default|GetOnwer)) (Variables|Default|GetRadius) (Utilities|Array|MakeArray "ObjectTypeQuery3") "/Game/MyWork/Characters/BP_BaseCharacter.BP_BaseCharacter_C"))
  ;[0.15 0.15 0.15 0.5] For each actor, check if they are an enemy
  (for _array_element _outactors
    (bind _actor_target_type (Class|BPITargeting|GetTargetType(Message) _array_element))
    ;[0.15 0.15 0.15 0.5] If they are, add to the Targets in Range array
    (if (Utilities|Enum|Equal(Enum) _actor_target_type "NewEnumerator2")
      (Utilities|Array|Add (Variables|Default|GetTargets%20in%20Range) _array_element)))
  (Utilities|IsValid _closest_actor
    (:Is%20Valid
      (Default|ApplyHealthChange _closest_actor (Variables|Default|GetHealing?) (Utilities|Struct|BreakS_StatusDefinition (Variables|Default|GetStatus%20Data))))))

(fn ConstructionScript
  (|CallParentFunction))

(fn FindClosestTarget
  (LocalVariables|SetL%20Closest%20Distance (Variables|Default|GetRadius))
  (for _array_element (Variables|Default|GetTargets%20in%20Range)
    (if (< (Transformation|GetDistanceTo (Variables|Default|GetOnwer) _array_element) (LocalVariables|GetL%20Closest%20Distance))
      (LocalVariables|SetL%20Closest%20Distance (Transformation|GetDistanceTo (Variables|Default|GetOnwer) _array_element))
      (bind _attribute_component (Class|BPIAttributeHandling|GetAttributeComponent(Message) _array_element))
      (LocalVariables|SetL%20Closest%20Taraget _attribute_component)))
  (return (LocalVariables|GetL%20Closest%20Taraget)))