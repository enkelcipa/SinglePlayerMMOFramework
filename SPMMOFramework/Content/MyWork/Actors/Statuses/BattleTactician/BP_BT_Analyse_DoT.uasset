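; Battle Tactician Analyse damage-over-time status that builds Tactical Prowess on its owner.
; Each proc and the status end grant one point of Tactical Prowess through the owner's attribute component.
; Refreshing also grants a point when the remaining duration is three or less, rewarding a late refresh.
; End and refresh then defer to the parent status logic.
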(event EventBeginPlay
  (|CallParentFunction) ; This node is disabled and will not be called.\nDrag off pins to build functionality.
)

(event Collision|EventActorBeginOverlap
  (params (OtherActor :type Actor%20Object%20Reference)))

(event EventTick
  (params (DeltaSeconds :type Float%20%28single-precision%29)))

(event EventApplyProcEffect
  (bind _attribute_component (Class|BPIAttributeHandling|GetAttributeComponent(Message) (Variables|Default|GetOnwer)))
  (Default|ApplyTacticalProwessChange _attribute_component true 1.0))

(event EventStatusEnd
  (bind _attribute_component (Class|BPIAttributeHandling|GetAttributeComponent(Message) (Variables|Default|GetOnwer)))
  (Default|ApplyTacticalProwessChange _attribute_component true 1.0)
  (|CallParentFunction))

(event EventRefreshStatus
  (if (<= (Variables|Default|GetDuration%20Remaining) 3)
    (bind _attribute_component (Class|BPIAttributeHandling|GetAttributeComponent(Message) (Variables|Default|GetOnwer)))
    (Default|ApplyTacticalProwessChange _attribute_component true 1.0)
    (|CallParentFunction)
    (else
      (|CallParentFunction))))

(fn ConstructionScript
  (|CallParentFunction))