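; BP_ZoneActor_Base is a base zone actor that applies damage or healing to actors inside its sphere.
; Sphere overlaps add actors that return a valid attribute component to ActorsToDamage and remove them when they leave.
; A looping one-second timer started on BeginPlay drives the periodic effect, with DamageActors passing the Healing and DamageToApply variables to each tracked actor's attribute component.
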(event OnComponentBeginOverlap(Sphere)
  (params (OverlappedComponent :type Primitive%20Component%20Object%20Reference) (OtherActor :type Actor%20Object%20Reference) (OtherComp :type Primitive%20Component%20Object%20Reference) (OtherBodyIndex :type Integer) (bFromSweep :type Boolean) (SweepResult :type Hit%20Result%20Structure%20%28by%20ref%29))
  (bind _attribute_component (Class|BPIAttributeHandling|GetAttributeComponent(Message) OtherActor))
  (Utilities|IsValid _attribute_component
    (:Is%20Valid
      (Utilities|Array|Add (Variables|Default|GetActors%20To%20Damage) OtherActor))))

(event OnComponentEndOverlap(Sphere)
  (params (OverlappedComponent :type Primitive%20Component%20Object%20Reference) (OtherActor :type Actor%20Object%20Reference) (OtherComp :type Primitive%20Component%20Object%20Reference) (OtherBodyIndex :type Integer))
  (bind _actors_to_damage (Variables|Default|GetActors%20To%20Damage))
  (Utilities|Array|RemoveIndex _actors_to_damage (Utilities|Array|FindItem _actors_to_damage OtherActor)))

(event Custom|Damage%20Actors
  (for _array_element (Variables|Default|GetActors%20To%20Damage)
    (bind _attribute_component (Class|BPIAttributeHandling|GetAttributeComponent(Message) _array_element))
    (Default|ApplyHealthChange _attribute_component (Variables|Default|GetHealing?) (Variables|Default|GetDamage%20To%20Apply))))

(event EventBeginPlay
  (bind _returnvalue (Utilities|Time|SetTimerbyEvent (EventDispatchers|CreateEvent :!event Custom|Damage%20Actors) 1.0 true))
  (Variables|Default|SetTimer%20Handle _returnvalue))

(fn ConstructionScript)