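; Actor component holding HP, MP, Aetherflow, Tactics Gauge and Tactical Prowess, with clamped changes broadcast through change events.
; ApplyResourceCosts routes by resource type; HP changes pass through multiplicative mitigations, healing included, then damage drains shields.
; Shields are insertion-sorted by ascending priority, and exclusive ones replace only weaker shields of their type.
; Depleted shields are removed in reverse index order along with their status.
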(event Custom|Init:%20Values
  (Variables|BasicAttributes|SetCurrent%20HP (Variables|BasicAttributes|GetMax%20HP))
  (Variables|BasicAttributes|SetCurrent%20MP (Variables|BasicAttributes|GetMax%20MP)))

(event Custom|Update%20Bars
  (Default|CallEvent:HPChange (Variables|BasicAttributes|GetCurrent%20HP) (Variables|BasicAttributes|GetMax%20HP))
  (Default|CallEvent:MPChange (Variables|BasicAttributes|GetCurrent%20MP) (Variables|BasicAttributes|GetMax%20MP))
  (Default|CallEvent:TacticsGaugeChange (Variables|TacticsGauge|GetCurrent%20Tactics%20Gauge) (Variables|TacticsGauge|GetMax%20Tactics%20Gauge))
  (Default|CallEvent:AetherflowChange (Variables|Aetherflow|GetCurrent%20Aetherflow) (Variables|Aetherflow|GetMax%20Aetherflow))
  (Default|CallEvent:TacticalProwessChange (Variables|TacticalProwess|GetCurrent%20Tactical%20Prowess) (Variables|TacticalProwess|GetMax%20Tactical%20Prowess)))

(event EventBeginPlay
  (CallFunction|Init:Values))

(fn ApplyHealthChange
  (params (Healing? :type Boolean) (Incoming%20Damage :type Float%20%28double-precision%29))
  (bind _mitigated_damage (Mitigation|CalculateMitigatedDamage Incoming%20Damage))
  (LocalVariables|SetL%20Damage%20To%20Apply _mitigated_damage)
  (if Healing?
    _
    (else
      (bind _remainder (Shielding|AbsorbDamage (LocalVariables|GetL%20Damage%20To%20Apply)))
      (bind _output_get (LocalVariables|SetL%20Damage%20To%20Apply _remainder))))
  (bind _output_get_2 (Variables|BasicAttributes|SetCurrent%20HP (Math|Float|Clamp(Float) (- (Variables|BasicAttributes|GetCurrent%20HP) (Math|Float|SelectFloat (* _output_get -1.0) _output_get Healing?)) 0.0 (Variables|BasicAttributes|GetMax%20HP))))
  (Default|CallEvent:HPChange _output_get_2 (Variables|BasicAttributes|GetMax%20HP)))

(fn ApplyManaChange
  (params (Increase? :type Boolean) (Change%20Amount :type Float%20%28double-precision%29))
  (bind _output_get (Variables|BasicAttributes|SetCurrent%20MP (Math|Float|Clamp(Float) (- (Variables|BasicAttributes|GetCurrent%20MP) (Math|Float|SelectFloat (* Change%20Amount -1.0) Change%20Amount Increase?)) 0.0 (Variables|BasicAttributes|GetMax%20MP))))
  (Default|CallEvent:MPChange _output_get (Variables|BasicAttributes|GetMax%20MP)))

(fn ApplyResourceCosts
  (params (Resource :type E_Resources%20Enum :default "NewEnumerator2") (Increase? :type Boolean) (Cost :type Float%20%28double-precision%29))
  (switch Utilities|FlowControl|Switch|SwitchonE_Resources Resource
    (:NewEnumerator2
      (return))
    (:NewEnumerator0
      (BasicAttributes|ApplyHealthChange Increase? Cost))
    (:NewEnumerator1
      (BasicAttributes|ApplyManaChange Increase? Cost))
    (:NewEnumerator3
      (ClassResources|ApplyAetherflowChange Increase? Cost))
    (:NewEnumerator4
      (ClassResources|ApplyTacticsGaugeChange Increase? Cost))
    (:NewEnumerator5
      (ClassResources|ApplyTacticalProwessChange Increase? Cost))))

(fn TryAddShield
  (params (Shield%20to%20Add :type S%20Shield%20Instance%20Structure) (Override%20Shield%20Potency? :type Boolean) (Override%20Shield%20Potency :type Float%20%28double-precision%29))
  (if (Utilities|Struct|BreakS_ShieldInstance Shield%20to%20Add)
    (for _array_element (Variables|BasicAttributes|GetActive%20Shields)
      (LocalVariables|SetL%20Active%20Shield%20in%20Context _array_element)
      (if (Utilities|Enum|Equal(Enum) (Utilities|Struct|BreakS_ShieldInstance _array_element) (Utilities|Struct|BreakS_ShieldInstance Shield%20to%20Add))
        (LocalVariables|SetL%20Shield%20Found? true)
        (if (< (Utilities|Struct|BreakS_ShieldInstance (LocalVariables|GetL%20Active%20Shield%20in%20Context)) (Math|Float|SelectFloat Override%20Shield%20Potency (Utilities|Struct|BreakS_ShieldInstance Shield%20to%20Add) Override%20Shield%20Potency?))
          (Shielding|RemoveShield (LocalVariables|GetL%20Active%20Shield%20in%20Context))
          (Shielding|AddShield Shield%20to%20Add Override%20Shield%20Potency? Override%20Shield%20Potency)
          (Shielding|SortActiveShieldsbyPriority))))
    (LocalVariables|GetL%20Shield%20Found?
      (:then)
      (:else
        _)))
  (Shielding|AddShield Shield%20to%20Add Override%20Shield%20Potency? Override%20Shield%20Potency)
  (Shielding|SortActiveShieldsbyPriority))

(fn AddShield
  (params (Shield%20to%20Add :type S%20Shield%20Instance%20Structure) (Override%20Shield%20Potency? :type Boolean) (Override%20Shield%20Potency :type Float%20%28double-precision%29))
  (LocalVariables|SetL%20Shield%20to%20Add Shield%20to%20Add)
  (if Override%20Shield%20Potency?
    (bind _structout (Utilities|Struct|SetmembersinS_ShieldInstance (LocalVariables|GetL%20Shield%20to%20Add) Override%20Shield%20Potency Override%20Shield%20Potency))
    (Utilities|Array|Add (Variables|BasicAttributes|GetActive%20Shields) _structout)
    (else
      (Utilities|Array|Add (Variables|BasicAttributes|GetActive%20Shields) (LocalVariables|GetL%20Shield%20to%20Add)))))

(fn RemoveShield
  (params (Shield%20to%20Remove :type S%20Shield%20Instance%20Structure))
  ;[0.15 0.15 0.15 0.5] Remove the old shield status
  (bind _status_component (Class|BPIStatusHandling|GetStatusComponent(Message) (Components|GetOwner)))
  (Default|RemoveStatus _status_component (Utilities|Struct|BreakS_ShieldInstance Shield%20to%20Remove))
  ;[0.15 0.15 0.15 0.5] Remove from Active Shields
  (Utilities|Array|RemoveItem (Variables|BasicAttributes|GetActive%20Shields) Shield%20to%20Remove))

(fn AbsorbDamage
  (params (Incoming%20Damage :type Float%20%28double-precision%29))
  (LocalVariables|SetL%20Remaining%20Damage Incoming%20Damage)
  (Utilities|Array|Clear (LocalVariables|GetIndices%20to%20Remove))
  ;[0.15 0.15 0.15 0.5] For each active shield, check if Remaining Damage is greater than or equal to 0, if True then break out of the loop
  (bind (_array_element _array_index) (Utilities|Array|ForEachLoopwithBreak (Variables|BasicAttributes|GetActive%20Shields) :!label _label)
    (:LoopBody
      (if (<= (LocalVariables|GetL%20Remaining%20Damage) 0.0)
        (goto _label Break)
        (else
          ;[0.15 0.15 0.15 0.5] If the current shield value is greater than or equal to remaining damage
          (if (>= (Utilities|Struct|BreakS_ShieldInstance _array_element) (LocalVariables|GetL%20Remaining%20Damage))
            ;[0.15 0.15 0.15 0.5] Subtract remaining damage from current shield value and set it back in the struct
            (Utilities|Struct|SetmembersinS_ShieldInstance (Utilities|Array|Get(acopy) (Variables|BasicAttributes|GetActive%20Shields) _array_index) (- (Utilities|Struct|BreakS_ShieldInstance _array_element) (LocalVariables|GetL%20Remaining%20Damage)))
            ;[0.15 0.15 0.15 0.5] Set Remaining Damage to 0
            (LocalVariables|SetL%20Remaining%20Damage 0.0)
            (else
              ;[0.15 0.15 0.15 0.5] Subtract Current Value of Shield from Remaining Damage and set Current Value to 0
              (LocalVariables|SetL%20Remaining%20Damage (- (LocalVariables|GetL%20Remaining%20Damage) (Utilities|Struct|BreakS_ShieldInstance _array_element)))
              (Utilities|Struct|SetmembersinS_ShieldInstance (Utilities|Array|Get(acopy) (Variables|BasicAttributes|GetActive%20Shields) _array_index) 0.0)))
          ;[0.15 0.15 0.15 0.5] If the Current Value of the shield in current loop is 0
          (if (== (Utilities|Struct|BreakS_ShieldInstance _array_element) 0.0)
            ;[0.15 0.15 0.15 0.5] Add it to Indices To Remove
            (Utilities|Array|Add (LocalVariables|GetIndices%20to%20Remove) _array_index)))))
    (:Completed
      (Utilities|Array|Reverse (LocalVariables|GetIndices%20to%20Remove))
      (for _array_element_2 (LocalVariables|GetIndices%20to%20Remove)
        (Shielding|RemoveShield (Utilities|Array|Get(acopy) (Variables|BasicAttributes|GetActive%20Shields) _array_element_2)))
      (return (LocalVariables|GetL%20Remaining%20Damage)))))

(fn SortActiveShieldsbyPriority
  (for _index (range 1 (- (Utilities|Array|Length (Variables|BasicAttributes|GetActive%20Shields)) 1))
    (bind _output_get (LocalVariables|SetL%20i _index))
    (bind _output_get_2 (LocalVariables|SetL%20j _output_get))
    (if (and (> _output_get_2 0) (< (Utilities|Struct|BreakS_ShieldInstance (Utilities|Array|Get(acopy) (Variables|BasicAttributes|GetActive%20Shields) (LocalVariables|GetL%20j))) (Utilities|Struct|BreakS_ShieldInstance (Utilities|Array|Get(acopy) (Variables|BasicAttributes|GetActive%20Shields) (- (LocalVariables|GetL%20j) 1))))) :!label _label
      (LocalVariables|SetL%20Temp (Utilities|Array|Get(acopy) (Variables|BasicAttributes|GetActive%20Shields) (LocalVariables|GetL%20j)))
      (Utilities|Array|SetArrayElem (Variables|BasicAttributes|GetActive%20Shields) (LocalVariables|GetL%20j) (Utilities|Array|Get(acopy) (Variables|BasicAttributes|GetActive%20Shields) (- (LocalVariables|GetL%20j) 1)))
      (Utilities|Array|SetArrayElem (Variables|BasicAttributes|GetActive%20Shields) (- (LocalVariables|GetL%20j) 1) (LocalVariables|GetL%20Temp))
      (LocalVariables|SetL%20j (- (LocalVariables|GetL%20j) 1))
      (goto _label))))

(fn ApplyTacticsGaugeChange
  (params (Increase? :type Boolean) (Change%20Amount :type Float%20%28double-precision%29))
  (bind _output_get (Variables|TacticsGauge|SetCurrent%20Tactics%20Gauge (Math|Float|Clamp(Float) (- (Variables|TacticsGauge|GetCurrent%20Tactics%20Gauge) (Math|Float|SelectFloat (* Change%20Amount -1.0) Change%20Amount Increase?)) 0.0 (Variables|TacticsGauge|GetMax%20Tactics%20Gauge))))
  (Default|CallEvent:TacticsGaugeChange _output_get (Variables|TacticsGauge|GetMax%20Tactics%20Gauge)))

(fn ApplyAetherflowChange
  (params (Increase? :type Boolean) (Change%20Amount :type Float%20%28double-precision%29))
  (bind _output_get (Variables|Aetherflow|SetCurrent%20Aetherflow (Math|Float|Clamp(Float) (- (Variables|Aetherflow|GetCurrent%20Aetherflow) (Math|Float|SelectFloat (* Change%20Amount -1.0) Change%20Amount Increase?)) 0.0 (Variables|Aetherflow|GetMax%20Aetherflow))))
  (Default|CallEvent:AetherflowChange _output_get (Variables|Aetherflow|GetMax%20Aetherflow)))

(fn ApplyTacticalProwessChange
  (params (Increase? :type Boolean) (Change%20Amount :type Float%20%28double-precision%29))
  (bind _output_get (Variables|TacticalProwess|SetCurrent%20Tactical%20Prowess (Math|Float|Clamp(Float) (- (Variables|TacticalProwess|GetCurrent%20Tactical%20Prowess) (Math|Float|SelectFloat (* Change%20Amount -1.0) Change%20Amount Increase?)) 0.0 (Variables|TacticalProwess|GetMax%20Tactical%20Prowess))))
  (Default|CallEvent:TacticalProwessChange _output_get (Variables|TacticalProwess|GetMax%20Tactical%20Prowess)))

(fn AddMitigation
  (params (Multiplier :type Float%20%28double-precision%29) (Source :type Actor%20Object%20Reference))
  (Utilities|Array|Add (Variables|Default|GetActive%20Mitigations) (Utilities|Struct|MakeS_MitigationInstance Multiplier Source)))

(fn RemoveMitigation
  (params (Source :type Actor%20Object%20Reference))
  (for (_array_element _array_index) (Variables|Default|GetActive%20Mitigations)
    (if (== (Utilities|Struct|BreakS_MitigationInstance _array_element) Source)
      (Utilities|Array|RemoveIndex (Variables|Default|GetActive%20Mitigations) _array_index))))

(fn CalculateMitigatedDamage
  (params (Incoming%20Damage :type Float%20%28double-precision%29))
  (LocalVariables|SetL%20Damage%20Multiplier 1.0)
  (for _array_element (Variables|Default|GetActive%20Mitigations)
    (LocalVariables|SetL%20Damage%20Multiplier (* (LocalVariables|GetL%20Damage%20Multiplier) (Utilities|Struct|BreakS_MitigationInstance _array_element))))
  (return (* Incoming%20Damage (LocalVariables|GetL%20Damage%20Multiplier))))