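; Character ability component that handles activation, casting, global and per-ability cooldowns, and resource costs.
; TryActivateAbility looks up the ability by name, validates target, cast state, cooldown and cost, then StartCast branches on GCD, oGCD or unique-GCD type.
; Instant or timer-completed casts deduct cost and spawn the ability class as an actor initialized with owner and target.
; A looping timer, started on BeginPlay, advances cooldown, GCD and cast progress, broadcasting updates.
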(event Custom|Try%20Activate%20Ability
  (params (Ability%20in%20Slot :type Text))
  ;[0.15 0.15 0.15 0.5] Try Activate Ability
  (bind (_ability_found_ _ability_class) (CallFunction|GetAbilitybyName Ability%20in%20Slot))
  (if _ability_found_
    (Variables|Context|SetAbility%20in%20Context _ability_class)
    (if (CallFunction|CheckTarget)
      (if (Variables|CastTracking|GetIs%20Casting?)
        (Development|PrintString "Currently Casting")
        (else
          (switch Utilities|FlowControl|Switch|SwitchonE_CooldownType (Utilities|GetClassDefaults (Variables|Context|GetAbility%20in%20Context))
            (:NewEnumerator0
              (if (or (CallFunction|OnCooldown?) (Variables|GCD|GetGCD%20Active?)) :!label _label
                (Development|PrintString "GCD is Rolling or Ability on Cooldown")
                (else
                  (if (CallFunction|CheckResourceCost) :!label _label_2
                    (Variables|ActiveAbility|SetAbility%20to%20Cast (Variables|Context|GetAbility%20in%20Context))
                    (Variables|ActiveAbility|SetTarget%20for%20Ability (Variables|References|GetCurrent%20Target))
                    (CallFunction|StartCast)
                    (else
                      (Development|PrintString "Insufficient Resource"))))))
            (:NewEnumerator1
              (if (CallFunction|OnCooldown?)
                (Development|PrintString "oGCD on Cooldown")
                (else
                  (goto _label_2))))
            (:NewEnumerator2
              (goto _label)))))
      (else
        (Development|PrintString "Invalid Target")))
    (else
      (Development|PrintString "Ability Not Found in Data Table"))))

(event Custom|Activate%20Ability
  ;[0.15 0.15 0.15 0.5] Activate Ability Event
  (Variables|CastTracking|SetIs%20Casting? false)
  (Variables|CastTracking|SetCast%20Elapsed 0.0)
  (Default|CallEvent:CastUpdated "NewEnumerator1" 0.0 0.0)
  (CallFunction|ApplyResourceCosts)
  (bind _returnvalue (Game|SpawnActorfromClass (Variables|ActiveAbility|GetAbility%20to%20Cast) (Transformation|GetActorTransform (Variables|References|GetOwner)) "AlwaysSpawn" "MultiplyWithRoot" 0 0))
  (Default|Init:Ability _returnvalue (Variables|References|GetOwner) (Variables|ActiveAbility|GetTarget%20for%20Ability))
  (Variables|ActiveAbility|SetAbility%20to%20Cast 0)
  (Variables|Context|SetAbility%20Name%20in%20Context "None"))

(event Custom|Start%20Cast
  (bind _ability_to_cast (Variables|ActiveAbility|GetAbility%20to%20Cast))
  (bind _ability_to_cast_2 (Variables|ActiveAbility|GetAbility%20to%20Cast))
  (bind _ability_to_cast_3 (Variables|ActiveAbility|GetAbility%20to%20Cast))
  (bind (_ability_name _cooldown) (Utilities|GetClassDefaults _ability_to_cast))
  (bind (_ability_name_2 _cast_time _cooldown_type) (Utilities|GetClassDefaults _ability_to_cast_2))
  (bind (_ability_name_3 _cooldown_2) (Utilities|GetClassDefaults _ability_to_cast_3))
  ;[0.15 0.15 0.15 0.5] Start Cast
  (Variables|Context|SetAbility%20Name%20in%20Context _ability_name_2)
  (Variables|CastTracking|SetCast%20Duration _cast_time)
  (switch Utilities|FlowControl|Switch|SwitchonE_CooldownType _cooldown_type
    (:NewEnumerator0
      (Variables|GCD|SetGCD%20Active? true :!label _label)
      (bind _returnvalue (Utilities|Time|SetTimerbyEvent (EventDispatchers|CreateEvent :!event Custom|GCD%20Complete) (Variables|GCD|GetGCD%20Duration)))
      (Variables|GCD|SetGCD%20Timer%20Handle _returnvalue)
      (if (> (Variables|CastTracking|GetCast%20Duration) 0.0)
        (Variables|CastTracking|SetIs%20Casting? true)
        (bind _returnvalue_2 (Utilities|Time|SetTimerbyEvent (EventDispatchers|CreateEvent :!event Custom|Activate%20Ability) (Variables|CastTracking|GetCast%20Duration)))
        (Variables|CastTracking|SetCast%20Timer%20Handle _returnvalue_2)
        (Default|CallEvent:CastUpdated "NewEnumerator3" 0.0 (Variables|CastTracking|GetCast%20Duration) (Variables|Context|GetAbility%20Name%20in%20Context))
        (else
          (CallFunction|ActivateAbility))))
    (:NewEnumerator1
      (Utilities|Map|Add (Variables|Cooldowns|GetCooldown%20Map) _ability_name_3 _cooldown_2)
      (Utilities|Map|Add (Variables|Cooldowns|GetCooldown%20Remaining%20Map) _ability_name_3 _cooldown_2)
      (Default|CallEvent:CooldownUpdated _ability_name_3 _cooldown_2 _cooldown_2)
      (CallFunction|ActivateAbility))
    (:NewEnumerator2
      (Utilities|Map|Add (Variables|Cooldowns|GetCooldown%20Map) _ability_name _cooldown)
      (Utilities|Map|Add (Variables|Cooldowns|GetCooldown%20Remaining%20Map) _ability_name _cooldown)
      (Default|CallEvent:CooldownUpdated _ability_name _cooldown _cooldown)
      (goto _label))))

(event Custom|GCD%20Complete
  (bind _gcd_duration (Variables|GCD|GetGCD%20Duration))
  ;[0.15 0.15 0.15 0.5] GCD Complete
  (Variables|GCD|SetGCD%20Active? false)
  (Variables|GCD|SetGCD%20Elapsed 0.0)
  (Default|CallEvent:GCDChanged false _gcd_duration _gcd_duration))

(event Custom|Ability%20Failed
  ;[0.15 0.15 0.15 0.5] Ability Failed
  (Variables|CastTracking|GetIs%20Casting?
    (:then
      (Utilities|Time|ClearandInvalidateTimerbyHandle (Variables|CastTracking|GetCast%20Timer%20Handle))
      (Utilities|Time|ClearandInvalidateTimerbyHandle (Variables|GCD|GetGCD%20Timer%20Handle))
      (Variables|GCD|SetGCD%20Active? false)
      (Variables|CastTracking|SetIs%20Casting? false)
      (Variables|CastTracking|SetCast%20Elapsed 0.0)
      (Variables|GCD|SetGCD%20Elapsed 0.0)
      (Variables|ActiveAbility|SetAbility%20to%20Cast 0)
      (Variables|Context|SetAbility%20Name%20in%20Context "None")
      (Default|CallEvent:AbilityFailed))
    (:else)))

(event Custom|Tick
  ;[0.15 0.15 0.15 0.5] Tick Event
  (Utilities|FlowControl|Sequence
    (:then_0
      ;;[0.15 0.15 0.15 0.5] Cooldown tracking
      (bind (_keypin _valuepin) (Utilities|Map|ForEachLoop(Map) (Variables|Cooldowns|GetCooldown%20Remaining%20Map))
        (:then
          (Variables|Context|SetAbility%20Name%20in%20Context _keypin)
          (bind _output_get (Variables|Context|SetTime%20Remaining%20in%20Context (- _valuepin (Variables|Default|GetTick%20Frequency))))
          (if (<= _output_get 0.0)
            ;;[0.15 0.15 0.15 0.5] Remove from the maps that track the cooldowns
            (Utilities|Map|Remove (Variables|Cooldowns|GetCooldown%20Remaining%20Map) (Variables|Context|GetAbility%20Name%20in%20Context))
            (Utilities|Map|Remove (Variables|Cooldowns|GetCooldown%20Map) (Variables|Context|GetAbility%20Name%20in%20Context))
            ;;[0.15 0.15 0.15 0.5] Broadcast update for UI
            (Default|CallEvent:CooldownUpdated (Variables|Context|GetAbility%20Name%20in%20Context) 0.0 (.Value (Utilities|Map|Find (Variables|Cooldowns|GetCooldown%20Map) (Variables|Context|GetAbility%20Name%20in%20Context))))
            (else
              ;;[0.15 0.15 0.15 0.5] Update cooldowns remaining duration
              (Utilities|Map|Add (Variables|Cooldowns|GetCooldown%20Remaining%20Map) (Variables|Context|GetAbility%20Name%20in%20Context) (Variables|Context|GetTime%20Remaining%20in%20Context))
              ;;[0.15 0.15 0.15 0.5] Broadcast Update for UI
              (Default|CallEvent:CooldownUpdated (Variables|Context|GetAbility%20Name%20in%20Context) (Variables|Context|GetTime%20Remaining%20in%20Context) (.Value (Utilities|Map|Find (Variables|Cooldowns|GetCooldown%20Map) (Variables|Context|GetAbility%20Name%20in%20Context)))))))))
    (:then_1
      ;;[0.15 0.15 0.15 0.5] GCD Tracking
      (if (Variables|GCD|GetGCD%20Active?)
        (bind _output_get_2 (Variables|GCD|SetGCD%20Elapsed (+ (Variables|GCD|GetGCD%20Elapsed) (Variables|Default|GetTick%20Frequency))))
        (Default|CallEvent:GCDChanged true _output_get_2 (Variables|GCD|GetGCD%20Duration))))
    (:then_2
      ;;[0.15 0.15 0.15 0.5] Cast Time Updates
      (if (Variables|CastTracking|GetIs%20Casting?)
        (bind _output_get_3 (Variables|CastTracking|SetCast%20Elapsed (+ (Variables|CastTracking|GetCast%20Elapsed) (Variables|Default|GetTick%20Frequency))))
        (Default|CallEvent:CastUpdated "NewEnumerator0" _output_get_3 (Variables|CastTracking|GetCast%20Duration) (Utilities|GetClassDefaults (Variables|Context|GetAbility%20in%20Context)))))))

(event EventBeginPlay
  ;[0.15 0.15 0.15 0.5] Get Owner and Attributes Component
  (bind _ascharacter (Utilities|Casting|CastToCharacter (Components|GetOwner)))
  (bind _output_get (Variables|References|SetOwner _ascharacter))
  (bind _attribute_component (Class|BPIAttributeHandling|GetAttributeComponent(Message) _output_get))
  (Variables|References|SetAttributes _attribute_component)
  (bind _returnvalue (Utilities|Time|SetTimerbyEvent (EventDispatchers|CreateEvent :!event Custom|Tick) (Variables|Default|GetTick%20Frequency) true))
  (Variables|Default|SetTick%20Timer _returnvalue))

(fn OnCooldown?
  (return (Utilities|Map|Contains (Variables|Cooldowns|GetCooldown%20Remaining%20Map) (.Ability%20Name (Utilities|GetClassDefaults (Variables|Context|GetAbility%20in%20Context))))))

(fn CheckResourceCost
  (bind _ability_in_context (Variables|Context|GetAbility%20in%20Context))
  (bind (_resource_type _resource_cost) (Utilities|GetClassDefaults _ability_in_context))
  (bind _current_value (Class|BPIAttributeHandling|GetCurrentResourceValue(Message) (Variables|References|GetOwner) _resource_type))
  (return (>= _current_value _resource_cost)))

(fn ApplyResourceCosts
  (bind _ability_to_cast (Variables|ActiveAbility|GetAbility%20to%20Cast))
  (bind (_resource_type _resource_cost) (Utilities|GetClassDefaults _ability_to_cast))
  (if (Utilities|IsValidClass _ability_to_cast)
    (Default|ApplyResourceCosts (Variables|References|GetAttributes) _resource_type _resource_cost)))

(fn CheckTarget
  (if (Utilities|Array|ContainsItem (Utilities|GetClassDefaults (Variables|Context|GetAbility%20in%20Context)) "NewEnumerator6")
    (return true)
    (else
      (Utilities|IsValid (Variables|References|GetCurrent%20Target)
        (:Is%20Valid
          (bind _actor_target_type (Class|BPITargeting|GetTargetType(Message) (Variables|References|GetCurrent%20Target)))
          (if (Utilities|Array|ContainsItem (Utilities|GetClassDefaults (Variables|Context|GetAbility%20in%20Context)) _actor_target_type)
            (return true)
            (else
              (return false))))
        (:Is%20Not%20Valid
          (if (Utilities|Array|ContainsItem (Utilities|GetClassDefaults (Variables|Context|GetAbility%20in%20Context)) "NewEnumerator0")
            (Variables|References|SetCurrent%20Target (Variables|References|GetOwner))
            (return true)
            (else
              (return false))))))))