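; Actor component that manages status effects on its owning Character, handling application, refresh, ticking and removal.
; Each status is an actor spawned and attached to the owner; reapplying one follows its refresh policy (refresh, stack or ignore), except Shield-tagged statuses, which always add a new instance.
; A looping timer drives duration ticks and removes statuses whose remaining duration reaches -1.
; Events broadcast when statuses are applied, updated or removed.
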(event Custom|Tick%20Statuses
  (for _array_element (Variables|Status|GetActive%20Statuses)
    (Utilities|IsValid _array_element
      (:Is%20Valid
        (Default|TickStatusDuration _array_element)
        (Default|CallEvent:StatusUpdated _array_element (Variables|/Game/MyWork/Actors/Statuses/Base/BP_Status_Base.BP_Status_Base_C|GetDuration%20Remaining _array_element))
        (if (== (Variables|/Game/MyWork/Actors/Statuses/Base/BP_Status_Base.BP_Status_Base_C|GetDuration%20Remaining _array_element) -1)
          (CallFunction|RemoveStatus _array_element))))))

(event EventBeginPlay
  (bind _ascharacter (Utilities|Casting|CastToCharacter (Components|GetOwner)))
  (Variables|Owner|SetOwner _ascharacter)
  (bind _returnvalue (Utilities|Time|SetTimerbyEvent (EventDispatchers|CreateEvent :!event Custom|Tick%20Statuses) 1.0 true))
  (Variables|Default|SetTick%20Status'%20Timer _returnvalue))

(fn TryApplyStatus
  (params (Status%20to%20Apply :type BP%20Status%20Base%20Class%20Reference) (Instigator :type Character%20Object%20Reference) (Override%20Shield%20Potency? :type Boolean) (Override%20Shield%20Potency :type Float%20%28double-precision%29))
  ;[0.15 0.15 0.15 0.5] Does the status exist?
  (for _array_element (Variables|Status|GetActive%20Statuses)
    (if (== (Utilities|GetClass _array_element) Status%20to%20Apply)
      (if (Utilities|Array|ContainsItem (Utilities|Struct|BreakS_StatusDefinition (Variables|/Game/MyWork/Actors/Statuses/Base/BP_Status_Base.BP_Status_Base_C|GetStatus%20Data _array_element)) "Shield")
        (CallFunction|ApplyStatus Status%20to%20Apply Instigator Override%20Shield%20Potency? Override%20Shield%20Potency)
        (return true)
        (else
          (bind _success_ (CallFunction|RefreshStatus _array_element))
          (return _success_)))))
  ;[0.15 0.15 0.15 0.5] If it doesn't, apply the status
  (CallFunction|ApplyStatus Status%20to%20Apply Instigator Override%20Shield%20Potency? Override%20Shield%20Potency)
  (return true))

(fn RefreshStatus
  (params (Status%20to%20Refresh :type BP%20Status%20Base%20Object%20Reference))
  (switch Utilities|FlowControl|Switch|SwitchonE_StatusRefreshPolicy (Utilities|Struct|BreakS_StatusDefinition (Variables|/Game/MyWork/Actors/Statuses/Base/BP_Status_Base.BP_Status_Base_C|GetStatus%20Data Status%20to%20Refresh))
    (:NewEnumerator0
      (Default|RefreshStatus Status%20to%20Refresh)
      (return true))
    (:NewEnumerator3
      (Default|IncreaseStacks Status%20to%20Refresh)
      (return true))
    (:NewEnumerator2
      (return false))))

(fn ApplyStatus
  (params (Status%20to%20Apply :type BP%20Status%20Base%20Class%20Reference) (Status%20Instigator :type Character%20Object%20Reference) (Override%20Shield%20Potency? :type Boolean) (Override%20Shield%20Potency :type Float%20%28double-precision%29))
  (bind _returnvalue (Game|SpawnActorfromClass Status%20to%20Apply (Transformation|GetActorTransform (Variables|Owner|GetOwner)) "Undefined" "MultiplyWithRoot" 0 0))
  (Transformation|AttachActorToActor _returnvalue (Variables|Owner|GetOwner) "None" "KeepRelative" "KeepRelative" "KeepRelative" true)
  (Default|Init:Status _returnvalue Status%20Instigator (Components|GetOwner) Override%20Shield%20Potency? Override%20Shield%20Potency)
  (Utilities|Array|Add (Variables|Status|GetActive%20Statuses) _returnvalue)
  (Default|CallEvent:StatusApplied _returnvalue))

(fn RemoveStatus
  (params (Status%20to%20Remove :type BP%20Status%20Base%20Object%20Reference))
  (Utilities|Array|RemoveItem (Variables|Status|GetActive%20Statuses) Status%20to%20Remove)
  (Default|CallEvent:StatusRemoved Status%20to%20Remove)
  (Default|StatusEnd Status%20to%20Remove))